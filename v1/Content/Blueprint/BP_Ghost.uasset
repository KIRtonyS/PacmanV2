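; BP_Ghost is a Pac-Man-style ghost pawn that roams, chases the player and swaps between killer and prey.
; It loops AIMoveTo to random reachable points, switching to chasing on PawnSensing if Chaseplayer is set and resuming roaming when the chase fails.
; Overlap destroys the player, or the ghost while scared; Changemode triggers that timed state with a blue material.
; SetSlowMotion toggles the ghost's own time dilation from IsSlow.
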(event OnSeePawn(PawnSensing)
  (params (Pawn :type Pawn%20Object%20Reference))
  (if (Variables|Default|GetChaseplayer)
    (Development|PrintString "Chase")
    (bind _asbp_top_down_character (Utilities|Casting|CastToBP_TopDownCharacter (Game|GetPlayerCharacter 0)))
    (AI|AIMoveTo self "0, 0, 0" _asbp_top_down_character 5.0 false
      (:OnFail
        (Utilities|FlowControl|RetriggerableDelay 0.5)
        (CallFunction|RandomRoam)))))

(event OnComponentBeginOverlap(Sphere1)
  (params (OverlappedComponent :type Primitive%20Component%20Object%20Reference) (OtherActor :type Actor%20Object%20Reference) (OtherComp :type Primitive%20Component%20Object%20Reference) (OtherBodyIndex :type Integer) (bFromSweep :type Boolean) (SweepResult :type Hit%20Result%20Structure%20%28by%20ref%29))
  (bind _asbp_top_down_character (Utilities|Casting|CastToBP_TopDownCharacter OtherActor))
  (if (Variables|Default|GetIsScared?)
    (Actor|DestroyActor)
    (else
      (Actor|DestroyActor _asbp_top_down_character))))

(event Custom|Random%20Roam
  (AI|AIMoveTo self (.RandomLocation (AI|Navigation|GetRandomReachablePointinRadius (Transformation|GetActorLocation) 3e+03 0 0)) 0 5.0 false
    (:OnSuccess
      _)
    (:OnFail
      _))
  (CallFunction|RandomRoam))

(event Custom|Changemode
  (Variables|Default|SetIsScared? true)
  (Rendering|Material|SetMaterial (Variables|Default|Getghost) 0 "/Game/LevelPrototyping/Materials/MI_Solid_Blue.MI_Solid_Blue")
  (Utilities|FlowControl|Delay 5.0)
  (Variables|Default|SetIsScared? false)
  (Rendering|Material|SetMaterial (Variables|Default|Getghost) 0 "/Game/StarterContent/Materials/M_Basic_Wall.M_Basic_Wall"))

(event EventBeginPlay
  (Utilities|FlowControl|Delay 3.0)
  (CallFunction|RandomRoam))

(fn ConstructionScript)

(fn SetSlowMotion
  (if (Variables|Default|GetIsSlow?)
    (Variables|Default|SetCustomTimeDilation 0.3)
    (else
      (Variables|Default|SetCustomTimeDilation 1.0))))