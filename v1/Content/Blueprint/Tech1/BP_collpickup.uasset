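; Collectible pickup that a Player-tagged actor collects by overlapping its sphere, counting toward a win condition.
; Overlap increments CollectionNumber on BP_TopDownController, plays sound and shockwave effects, passes CollectionValue to AddtoCollection, and destroys the pickup.
; Reaching WinNumber pauses the game and shows WBP_Win with UI-only input.
; Disconnected nodes hold unused animation-speed and timed hide-and-reappear logic.
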(event OnComponentBeginOverlap(Sphere)
  (params (OverlappedComponent :type Primitive%20Component%20Object%20Reference) (OtherActor :type Actor%20Object%20Reference) (OtherComp :type Primitive%20Component%20Object%20Reference) (OtherBodyIndex :type Integer) (bFromSweep :type Boolean) (SweepResult :type Hit%20Result%20Structure%20%28by%20ref%29))
  (if (Actor|ActorHasTag OtherActor "Player")
    (bind _asbp_top_down_controller (Utilities|Casting|CastToBP_TopDownController (Game|GetPlayerController 0)))
    (Variables|/Game/TopDown/Blueprints/BP_TopDownController.BP_TopDownController_C|SetCollectionNumber _asbp_top_down_controller (+ (Variables|/Game/TopDown/Blueprints/BP_TopDownController.BP_TopDownController_C|GetCollectionNumber _asbp_top_down_controller) 1))
    (Audio|PlaySoundatLocation "/Game/Sound/pick_up.pick_up" (Transformation|GetWorldLocation (Variables|Default|GetSphere)) "0, 0, 0" 1.0 1.0 0.0 0 0 0 0)
    (Effects|SpawnEmitteratLocation "/Game/FXVarietyPack/Particles/P_ky_shotShockwave.P_ky_shotShockwave" (Transformation|GetWorldLocation (Variables|Default|GetSphere)))
    (bind _asbp_top_down_controller_2 (Utilities|Casting|CastToBP_TopDownController (Game|GetPlayerController 0)))
    (Default|AddtoCollection _asbp_top_down_controller_2 (Variables|Default|GetCollectionValue))
    (Actor|DestroyActor)
    ;[0.15 0.15 0.15 0.5] Win
    (if (>= (Variables|/Game/TopDown/Blueprints/BP_TopDownController.BP_TopDownController_C|GetCollectionNumber _asbp_top_down_controller) (Variables|Default|GetWinNumber))
      (Game|SetGamePaused true)
      (Input|SetInputModeUIOnly (Game|GetPlayerController 0) 0 "DoNotLock" false)
      (bind _returnvalue (UserInterface|CreateWidget "/Game/InterfaceBluePrint/WBP_Win.WBP_Win_C"))
      (UserInterface|Viewport|AddtoViewport _returnvalue 0)
      (Default|FocusDefaultButton _returnvalue))))

(fn ConstructionScript)