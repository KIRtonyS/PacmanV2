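; Spawn manager that spawns BP_Ghost enemies at the world location of its Box component.
; A non-looping timer set on BeginPlay runs Check once after one second, pruning invalid entries from the AIActor array before calling EnemySpawn.
; Despite a length check against four, the loop bounds spawn a single ghost only when the array is empty, then add it to the array.
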(event Custom|Check
  (for (_array_element _array_index) (Variables|Default|GetAI%20actor)
    (Utilities|IsValid _array_element
      (:Is%20Not%20Valid
        (Utilities|Array|RemoveIndex (Variables|Default|GetAI%20actor) _array_index))))
  (CallFunction|EnemySpawn))

(event Custom|EnemySpawn
  (bind _ai_actor (Variables|Default|GetAI%20actor))
  (bind _returnvalue (Utilities|Array|Length _ai_actor))
  (if (< _returnvalue 4)
    (for _index (range 1 (- 1 _returnvalue))
      (bind _returnvalue_2 (Game|SpawnActorfromClass "/Game/Blueprint/BP_Ghost.BP_Ghost_C" (Math|Transform|MakeTransform (Transformation|GetWorldLocation (Variables|Default|GetBox)) "0, 0, 0" "1.000000,1.000000,1.000000") "Undefined" "MultiplyWithRoot" 0 true 0))
      (Utilities|Array|Add (Variables|Default|GetAI%20actor) _returnvalue_2))))

(event EventBeginPlay
  (Utilities|Time|SetTimerbyEvent (delegate Custom|Check) 1.0))

(fn ConstructionScript)