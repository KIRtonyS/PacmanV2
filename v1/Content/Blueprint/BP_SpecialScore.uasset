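; Timed bonus pickup whose cube appears once for a short window and awards bonus score to the player.
; On BeginPlay it hides the cube, waits a random delay, reveals it with a WBP_SpecialScore widget, then hides both after a fixed time.
; Overlap by a Player-tagged actor updates BP_TopDownController's count and score, plays effects, destroys the pickup and removes the widget.
; Hiding changes only visibility; overlap is not gated by it.
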(event OnComponentBeginOverlap(Cube)
  (params (OverlappedComponent :type Primitive%20Component%20Object%20Reference) (OtherActor :type Actor%20Object%20Reference) (OtherComp :type Primitive%20Component%20Object%20Reference) (OtherBodyIndex :type Integer) (bFromSweep :type Boolean) (SweepResult :type Hit%20Result%20Structure%20%28by%20ref%29))
  (if (Actor|ActorHasTag OtherActor "Player")
    (bind _asbp_top_down_controller (Utilities|Casting|CastToBP_TopDownController (Game|GetPlayerController 0)))
    (Variables|/Game/TopDown/Blueprints/BP_TopDownController.BP_TopDownController_C|SetCollectionNumber _asbp_top_down_controller (+ (Variables|/Game/TopDown/Blueprints/BP_TopDownController.BP_TopDownController_C|GetCollectionNumber _asbp_top_down_controller) 1))
    (Audio|PlaySoundatLocation "/Game/Sound/pick_up.pick_up" (Transformation|GetWorldLocation (Variables|Default|GetCube)) "0, 0, 0" 1.0 1.0 0.0 0 0 0 0)
    (Effects|SpawnEmitteratLocation "/Game/FXVarietyPack/Particles/P_ky_shotShockwave.P_ky_shotShockwave" (Transformation|GetWorldLocation (Variables|Default|GetCube)))
    (bind _asbp_top_down_controller_2 (Utilities|Casting|CastToBP_TopDownController (Game|GetPlayerController 0)))
    (Default|AddtoCollection _asbp_top_down_controller_2 500)
    (Actor|DestroyActor)
    (Widget|RemovefromParent (stale EventBeginPlay _returnvalue))))

(event EventBeginPlay
  (Development|SetHiddeninGame (Variables|Default|GetCube) true false)
  (Utilities|FlowControl|Delay (Math|Conversions|ToFloat(Integer) (Math|Random|RandomIntegerinRange 10 30)))
  (Development|SetHiddeninGame (Variables|Default|GetCube) false false)
  (bind _returnvalue (UserInterface|CreateWidget "/Game/InterfaceBluePrint/WBP_SpecialScore.WBP_SpecialScore_C"))
  (UserInterface|Viewport|AddtoViewport _returnvalue 0)
  (Utilities|FlowControl|Delay 1e+01)
  (Development|SetHiddeninGame (Variables|Default|GetCube) true false)
  (Widget|RemovefromParent _returnvalue))

(fn ConstructionScript)